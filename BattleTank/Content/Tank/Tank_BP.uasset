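; Tank_BP is the player-controlled tank Blueprint, handling camera aiming and firing.
; On BeginPlay it passes its Barrel and TankTurret components to SetBarrelReference and SetTurretReference.
; AimAzimuth and AimElevation axes rotate the AzimuthGimbal yaw and SpringArm pitch, scaled by frame time, while the Fire action calls Fire.
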(event `self.ReceiveBeginPlay`
  (`self.SetBarrelReference` (`self.Barrel`))
  (`self.SetTurretReference` (`self.TankTurret`)))

(event `InputAxis|AimAzimuth`
  (params (AxisValue :type "Float (single-precision)"))
  (`SceneComponent.K2_AddLocalRotation` (`self.AzimuthGimbal`) (`KismetMathLibrary.MakeRotator` 0.0 0.0 (* AxisValue (`GameplayStatics.GetWorldDeltaSeconds`) 60.0)) false false))

(event `InputAxis|AimElevation`
  (params (AxisValue :type "Float (single-precision)"))
  (`SceneComponent.K2_AddLocalRotation` (`self.SpringArm`) (`KismetMathLibrary.MakeRotator` 0.0 (* AxisValue (`GameplayStatics.GetWorldDeltaSeconds`) 60.0)) false false))

(event `InputAction|Fire`
  (params (Key :type "Key Structure" :default "AnyKey"))
  (:`Pressed`
    (`self.Fire`)))

(fn `UserConstructionScript`)